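; BP_SelfActor is an input-enabled actor that fires BP_Shot1 actors and can be picked up.
; It enables input from player controller 0 on BeginPlay, then spawns shots at its root scene transform while the Shot axis is positive.
; ShotDistance counts those axis updates and wraps around, throttling fire by frame count rather than time.
; Pickup stops physics on Sphere1 and snaps the root onto the supplied component.
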(event `self.ReceiveBeginPlay`
  (`self.EnableInput` (`GameplayStatics.GetPlayerController` 0)))

(event `InputAxis|Shot`
  (params (AxisValue :type "Float (single-precision)"))
  (if (> AxisValue 0.0)
    (if (== (`self.shotDistance`) 0)
      (`|SpawnActorFromClass` "/Game/Progre/BP_Shot1.BP_Shot1_C" (`SceneComponent.K2_GetComponentToWorld` (`self.DefaultSceneRoot`)) "Undefined" "OverrideRootScale"))
    (bind _output_get (set `self.shotDistance` (+ (`self.shotDistance`) 1)))
    (if (> _output_get 10)
      (set `self.shotDistance` 0))))

(event `/Game/VirtualRealityBP/Blueprints/PickupActorInterface.Pickup`
  (params (AttachTo :type "SceneComponent Object Reference"))
  (`PrimitiveComponent.SetSimulatePhysics` (`self.Sphere1`) false)
  (`SceneComponent.K2_AttachToComponent` (`self.K2_GetRootComponent`) AttachTo "None" "SnapToTarget" "SnapToTarget" "SnapToTarget" false))

(fn `UserConstructionScript`)