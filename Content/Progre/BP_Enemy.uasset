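; Enemy actor that fires at random and drifts to line up with the player actor (BP_SelfActor).
; Each Tick has a small random chance to spawn a BP_Shot1 just in front, turned around and tagged as the enemy's.
; Tick also nudges the ProjectileMovement velocity toward the first BP_SelfActor on Y and Z only, using fixed per-frame steps, so tracking builds momentum and depends on frame rate.
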(event `self.ReceiveBeginPlay`)

(event `self.ReceiveTick`
  (params (DeltaSeconds :type "Float (single-precision)"))
  (bind _defaultsceneroot (`self.DefaultSceneRoot`))
  (`|ExecutionSequence`
    (:`then_0`
      ;[1 1 1] Shot
      (if (not (`KismetMathLibrary.Conv_IntToBool` (`KismetMathLibrary.RandomInteger` 100)))
        (bind _returnvalue (`|SpawnActorFromClass` "/Game/Progre/BP_Shot1.BP_Shot1_C" (`KismetMathLibrary.MakeTransform` (+ (`SceneComponent.K2_GetComponentLocation` _defaultsceneroot) (-10.0 0.0 0.0)) (struct :`Pitch` 180.0) (`SceneComponent.K2_GetComponentScale` _defaultsceneroot)) "Undefined" "OverrideRootScale"))
        (set `Actor.Tags` (`|MakeArray` "Enemy's" :!type "Name") _returnvalue)))
    (:`then_1`
      ;[1 1 1] Move
      (bind _outactors (`GameplayStatics.GetAllActorsOfClass` "/Game/Progre/BP_SelfActor.BP_SelfActor_C"))
      (bind _y (.y (- (`SceneComponent.K2_GetComponentLocation` (`self.DefaultSceneRoot`)) (`self.K2_GetActorLocation` (`KismetArrayLibrary.Array_Get` _outactors)))))
      (bind _z (.z (- (`SceneComponent.K2_GetComponentLocation` (`self.DefaultSceneRoot`)) (`self.K2_GetActorLocation` (`KismetArrayLibrary.Array_Get` _outactors)))))
      (`ProjectileMovementComponent.SetVelocityInLocalSpace` (`self.ProjectileMovement`) (+ (+ (+ (+ (`self.GetVelocity`) (select `bool` (< _y 0.0) :`true` (0.0 1.0 0.0) :!type "Vector Structure")) (select `bool` (> _y 0.0) :`true` (0.0 -1.0 0.0) :!type "Vector Structure")) (select `bool` (< _z 0.0) :`true` (0.0 0.0 1.0) :!type "Vector Structure")) (select `bool` (> _z 0.0) :`true` (0.0 0.0 -1.0) :!type "Vector Structure"))))))

(fn `UserConstructionScript`)