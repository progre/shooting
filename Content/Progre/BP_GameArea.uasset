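; BP_GameArea is a play-area actor that polices a boundary volume and restarts the level once all enemies are gone.
; While Started is set, Tick searches for BP_Enemy actors every frame and, when none remain, reloads the current level after a short Delay.
; The Cube1 overlap destroys incoming BP_Shot1 actors and teleports overlapping enemies by a fixed world offset along positive X.
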(event `self.ReceiveBeginPlay`)

(event `self.ReceiveTick`
  (params (DeltaSeconds :type "Float (single-precision)"))
  (if (`self.started`)
    (bind _outactors (`GameplayStatics.GetAllActorsOfClass` "/Game/Progre/BP_Enemy.BP_Enemy_C"))
    (if (<= (`KismetArrayLibrary.Array_Length` _outactors) 0)
      (`KismetSystemLibrary.Delay` 3.0)
      (bind _returnvalue (`GameplayStatics.GetCurrentLevelName` true))
      (`GameplayStatics.OpenLevel` (`KismetStringLibrary.Conv_StringToName` _returnvalue)))))

(event `self.Cube1.OnComponentBeginOverlap`
  (params (OverlappedComponent :type "PrimitiveComponent Object Reference") (OtherActor :type "Actor Object Reference") (OtherComp :type "PrimitiveComponent Object Reference") (OtherBodyIndex :type Integer) (bFromSweep :type Boolean) (SweepResult :type "HitResult Structure (by ref)"))
  (bind _asbp_shot_1 (cast `/Game/Progre/BP_Shot1` OtherActor)
    (:`then`
      (`self.K2_DestroyActor` _asbp_shot_1))
    (:`CastFailed`
      (bind _asbp_enemy (cast `/Game/Progre/BP_Enemy` OtherActor))
      (`SceneComponent.K2_AddWorldOffset` (`/Game/Progre/BP_Enemy.DefaultSceneRoot` _asbp_enemy) (200.0 0.0 0.0) false true))))

(fn `UserConstructionScript`)